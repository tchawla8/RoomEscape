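; Openable door actor that swings open and closed when its DoorOpen2 member raises open or close requests.
; The DoorSwing timeline plays on open and reverses on close, applying its OpenAngle as a yaw combined with the rotation cached at BeginPlay.
; A Sound Timing event track on the same timeline plays the Doorlock sound at the actor's location.
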(event OnOpenRequest(DoorOpen2)
  (bind _openangle (Timeline|DoorSwing Play)
    (:Update
      (Transformation|SetActorRotation (Math|Rotator|CombineRotators (Variables|Default|GetInitialRotation) (Math|Rotator|MakeRotator 0.0 0.0 _openangle))))
    (:Sound%20Timing
      (Audio|PlaySoundatLocation "/Game/Audio/door-lock.door-lock" (Transformation|GetActorLocation) "0, 0, 0" 1.0 1.0 0.0 0 0 0))))

(event OnCloseRequest(DoorOpen2)
  (bind _openangle (Timeline|DoorSwing Reverse)
    (:Update
      (Transformation|SetActorRotation (Math|Rotator|CombineRotators (Variables|Default|GetInitialRotation) (Math|Rotator|MakeRotator 0.0 0.0 _openangle))))
    (:Sound%20Timing
      (Audio|PlaySoundatLocation "/Game/Audio/door-lock.door-lock" (Transformation|GetActorLocation) "0, 0, 0" 1.0 1.0 0.0 0 0 0))))

(event EventBeginPlay
  (Variables|Default|SetInitialRotation (Transformation|GetActorRotation)))

(fn ConstructionScript)